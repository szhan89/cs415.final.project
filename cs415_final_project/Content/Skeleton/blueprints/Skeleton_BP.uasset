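; Skeleton enemy that patrols along the X axis, pausing and reversing when forward line traces detect an obstacle or a ledge.
; A player entering its Box starts a looping attack timer that plays the attack animation, while the Attack event traces ahead to apply damage.
; Incoming damage updates its health bar widget and turns it toward the attacker, then either knocks it back or plays death and destroys it.
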(event OnComponentBeginOverlap(Box)
  (params (OverlappedComponent :type Primitive%20Component%20Object%20Reference) (OtherActor :type Actor%20Object%20Reference) (OtherComp :type Primitive%20Component%20Object%20Reference) (OtherBodyIndex :type Integer) (bFromSweep :type Boolean) (SweepResult :type Hit%20Result%20Structure%20%28by%20ref%29))
  ;[1 1 1] Handle  Damage
  (if (== OtherActor (Game|GetPlayerCharacter 0))
    (Variables|Default|SetAttackmode true)
    (bind _returnvalue (Utilities|Time|SetTimerbyEvent (delegate Custom|Skeletonattack) 1.0 true))
    (Variables|Default|SetAttackEvent _returnvalue)))

(event OnComponentEndOverlap(Box)
  (params (OverlappedComponent :type Primitive%20Component%20Object%20Reference) (OtherActor :type Actor%20Object%20Reference) (OtherComp :type Primitive%20Component%20Object%20Reference) (OtherBodyIndex :type Integer))
  ;[1 1 1] Handle Attack System
  (if (== OtherActor (Game|GetPlayerCharacter 0))
    (Variables|Default|SetAttackmode false)
    (Utilities|Time|ClearandInvalidateTimerbyHandle (Variables|Default|GetAttackEvent))))

(event Custom|HandleMovemont
  (bind _returnvalue (Transformation|GetActorLocation))
  (bind _returnvalue_2 (Transformation|GetActorLocation))
  (if (not (Math|Boolean|ORBoolean (Variables|Default|GetisDead) (Variables|Default|GetenemyDamaged) (AI|Components|NavMovement|IsFalling (Variables|Character|GetCharacterMovement)) (Variables|Default|GetAttackmode)))
    (Pawn|Input|AddMovementInput "1.000000,0.000000,0.000000" (Variables|Default|GetMovementDirection) false)
    (Utilities|FlowControl|Sequence
      (:then_0
        ;[1 1 1] Detect if an object is on the front
        (bind _returnvalue_3 (Collision|LineTraceForObjects _returnvalue (+ _returnvalue (* (Transformation|GetActorForwardVector) (Math|Vector|MakeVector 1e+02 0.0 0.0))) (Utilities|Array|MakeArray "ObjectTypeQuery1" "ObjectTypeQuery2" "ObjectTypeQuery3") false (Utilities|Array|MakeArray (Game|GetPlayerCharacter 0)) "None"))
        (if _returnvalue_3
          (Utilities|FlowControl|DoOnce false :!label _label
            (:Completed
              (Variables|/Script/Engine.CharacterMovementComponent|SetMaxWalkSpeed (Variables|Character|GetCharacterMovement) 0.0)
              (Utilities|FlowControl|Delay (Variables|Default|GetwaitTime))
              (Variables|/Script/Engine.CharacterMovementComponent|SetMaxWalkSpeed (Variables|Character|GetCharacterMovement) (Variables|Default|GetMax%20Walk%20Speed))
              (Variables|Default|SetMovementDirection (* (Variables|Default|GetMovementDirection) -1.0))
              (goto _label Reset)))))
      (:then_1
        ;[1 1 1] edge detection
        (bind _returnvalue_4 (Collision|LineTraceForObjects _returnvalue_2 (+ (- _returnvalue_2 "0.000000,0.000000,100.000000") (* (Transformation|GetActorForwardVector) (Math|Vector|MakeVector 1e+02 0.0 0.0))) (Utilities|Array|MakeArray "ObjectTypeQuery1" "ObjectTypeQuery2" "ObjectTypeQuery3") false (Utilities|Array|MakeArray (Game|GetPlayerCharacter 0)) "None"))
        (if (not _returnvalue_4)
          (goto _label))))))

(event Custom|HandleRotation
  (if (> (Variables|Default|GetMovementDirection) 0.0)
    (Transformation|SetActorRotation "0, 0, 0")
    (else
      (Transformation|SetActorRotation "0.000000,180.000000,0.000000"))))

(event Custom|Skeletonattack
  ;[1 1 1] Handle  Damage
  (if (not (Variables|Default|GetisDead))
    (Class|PaperZDAnimInstance|JumptoNode (Variables|/Script/PaperZD.PaperZDAnimationComponent|GetAnimInstance (Variables|Default|GetAnimationComponent)) "AttackEvent" "None")))

(event Custom|Attack
  (bind _returnvalue (Transformation|GetActorLocation))
  ;[1 1 1] Handle Attack System
  (bind _outhit (Collision|LineTraceForObjects _returnvalue (+ _returnvalue (* (Transformation|GetActorForwardVector) (Math|Vector|MakeVector 1e+02 0.0 0.0))) (Utilities|Array|MakeArray "ObjectTypeQuery3") false 0 "None"))
  (if (== (.HitActor (Collision|BreakHitResult _outhit)) (Game|GetPlayerCharacter 0))
    (Game|Damage|ApplyDamage (.HitActor (Collision|BreakHitResult _outhit)) 1.0 0 0)))

(event EventBeginPlay
  (Variables|/Script/Engine.CharacterMovementComponent|SetMaxWalkSpeed (Variables|Character|GetCharacterMovement) 1e+02)
  (Variables|Default|SetmaxHealth (Variables|Default|GetHealth))
  (bind _asenemy_health_bar_widget (Utilities|Casting|CastToEnemyHealthBarWidget (UserInterface|GetWidget (Variables|Default|GetWidget))))
  (Variables|/Game/WidgeBlueprints/EnemyHealthBarWidget.EnemyHealthBarWidget_C|SetskeletonRef _asenemy_health_bar_widget self)
  (Variables|Default|SetAs%20Enemy%20Health%20Bar%20Widget _asenemy_health_bar_widget))

(event Collision|EventActorBeginOverlap
  (params (OtherActor :type Actor%20Object%20Reference)))

(event EventTick
  (params (DeltaSeconds :type Float%20%28single-precision%29))
  (CallFunction|HandleRotation)
  (CallFunction|HandleMovemont))

(event Game|Damage|EventAnyDamage
  (params (Damage :type Float%20%28single-precision%29) (DamageType :type Damage%20Type%20Object%20Reference) (InstigatedBy :type Controller%20Object%20Reference) (DamageCauser :type Actor%20Object%20Reference))
  (bind _returnvalue (Transformation|GetActorLocation DamageCauser))
  (bind _returnvalue_2 (Transformation|GetActorLocation))
  (bind _returnvalue_3 (Math|Vector|GetUnitDirection(Vector) _returnvalue _returnvalue_2))
  (bind _returnvalue_4 (< (.x _returnvalue_3) 0.0))
  (bind _returnvalue_5 (select _returnvalue_4 1.0 -1.0))
  (Variables|Default|SetHealth (- (Variables|Default|GetHealth) Damage))
  (Default|UpdateHealthBar (Variables|Default|GetAs%20Enemy%20Health%20Bar%20Widget))
  (Variables|Default|SetenemyDamaged true)
  (Variables|Default|SetMovementDirection _returnvalue_5)
  (if (<= (Variables|Default|GetHealth) 0.0)
    (Class|PaperZDAnimInstance|JumptoNode (Variables|/Script/PaperZD.PaperZDAnimationComponent|GetAnimInstance (Variables|Default|GetAnimationComponent)) "Death" "None")
    (Variables|Default|SetisDead true)
    (Collision|SetCollisionProfileName (Variables|Default|GetCapsuleComponent) "OverlapOnlyPawn" true :!class /Script/Engine.PrimitiveComponent)
    (Utilities|FlowControl|Delay 3.0)
    (Actor|DestroyActor)
    (else
      (Character|LaunchCharacter (Math|Vector|MakeVector (* _returnvalue_5 -8e+02) 0.0 1.5e+02) true true)
      (Class|PaperZDAnimInstance|JumptoNode (Variables|/Script/PaperZD.PaperZDAnimationComponent|GetAnimInstance (Variables|Default|GetAnimationComponent)) "Damage" "None")
      (Utilities|FlowControl|RetriggerableDelay 1.0)
      (Variables|Default|SetenemyDamaged false))))

(fn ConstructionScript)