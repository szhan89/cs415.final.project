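; Mushroom ranged enemy character that faces the player, fires projectiles and dies when its health runs out.
; Tick flips it toward the player, while a box overlap starts a looping attack timer gated on range, falling and death.
; Attacks and hit reactions jump animation nodes; a separate SpawnProjectile event spawns BossProjectile_BP at the spawn point.
; Damage updates the widget health bar and launches it away from the damage causer, or triggers death and delayed destruction.
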(event OnComponentBeginOverlap(Box)
  (params (OverlappedComponent :type Primitive%20Component%20Object%20Reference) (OtherActor :type Actor%20Object%20Reference) (OtherComp :type Primitive%20Component%20Object%20Reference) (OtherBodyIndex :type Integer) (bFromSweep :type Boolean) (SweepResult :type Hit%20Result%20Structure%20%28by%20ref%29))
  ;[1 1 1] Attack
  (if (== OtherActor (Game|GetPlayerCharacter 0))
    (Variables|Default|SetinRange true)
    (Utilities|Time|SetTimerbyEvent (delegate Custom|mushroomAttack) 1.0 true)))

(event OnComponentEndOverlap(Box)
  (params (OverlappedComponent :type Primitive%20Component%20Object%20Reference) (OtherActor :type Actor%20Object%20Reference) (OtherComp :type Primitive%20Component%20Object%20Reference) (OtherBodyIndex :type Integer))
  (Variables|Default|SetinRange false))

(event Custom|HandleRotation
  (if (not (Variables|Default|GetisDead))
    (if (< (.x (Math|Vector|GetUnitDirection(Vector) (Transformation|GetActorLocation (Game|GetPlayerCharacter 0)) (Transformation|GetActorLocation))) 0.0)
      (Transformation|SetActorRotation "0, 0, 0")
      (else
        (Transformation|SetActorRotation "0.000000,180.000000,0.000000")))))

(event Custom|mushroomAttack
  ;[1 1 1] Attack
  (if (not (Math|Boolean|ORBoolean (Variables|Default|GetisDead) (AI|Components|NavMovement|IsFalling (Variables|Character|GetCharacterMovement)) (not (Variables|Default|GetinRange))))
    (Class|PaperZDAnimInstance|JumptoNode (Variables|/Script/PaperZD.PaperZDAnimationComponent|GetAnimInstance (Variables|Default|GetAnimationComponent)) "attack" "None")))

(event Custom|SpawnProjectile
  ;[1 1 1] Attack
  (Game|SpawnActorfromClass "/Game/Mushroom/Blueprints/BossProjectile_BP.BossProjectile_BP_C" (Math|Transform|MakeTransform (Transformation|GetWorldLocation (Variables|Default|Getspawnpoint)) (Transformation|GetActorRotation) "1.000000,1.000000,1.000000") "Undefined" 0 0))

(event EventBeginPlay
  ;[1 1 1] EventBeginPlaySetUp
  (Variables|Default|SetmaxHealth (Variables|Default|GetHealth))
  (bind _asranged_enemy_health_bar_widget (Utilities|Casting|CastToRangedEnemyHealthBarWidget (UserInterface|GetWidget (Variables|Default|GetWidget))))
  (bind _output_get (Variables|Default|SetAs%20Ranged%20Enemy%20Health%20Bar _asranged_enemy_health_bar_widget))
  (Variables|/Game/WidgeBlueprints/RangedEnemyHealthBarWidget.RangedEnemyHealthBarWidget_C|SetMushroomRef _output_get self))

(event EventTick
  (params (DeltaSeconds :type Float%20%28single-precision%29))
  (CallFunction|HandleRotation))

(event Game|Damage|EventAnyDamage
  (params (Damage :type Float%20%28single-precision%29) (DamageType :type Damage%20Type%20Object%20Reference) (InstigatedBy :type Controller%20Object%20Reference) (DamageCauser :type Actor%20Object%20Reference))
  (Variables|Default|SetHealth (- (Variables|Default|GetHealth) Damage))
  (Default|UpdateHealthBar (Variables|Default|GetAs%20Ranged%20Enemy%20Health%20Bar))
  (Variables|Default|SetenemyDamaged true)
  (if (<= (Variables|Default|GetHealth) 0.0)
    (Class|PaperZDAnimInstance|JumptoNode (Variables|/Script/PaperZD.PaperZDAnimationComponent|GetAnimInstance (Variables|Default|GetAnimationComponent)) "mushroomdeath" "None")
    (Variables|Default|SetisDead true)
    (Rendering|SetVisibility (Variables|Default|GetWidget) false false)
    (Collision|SetCollisionProfileName (Variables|Default|GetCapsuleComponent) "OverlapOnlyPawn" true :!class /Script/Engine.PrimitiveComponent)
    (Utilities|FlowControl|Delay 3.0)
    (Actor|DestroyActor)
    (else
      (Character|LaunchCharacter (Math|Vector|MakeVector (* (select (< (.x (Math|Vector|GetUnitDirection(Vector) (Transformation|GetActorLocation DamageCauser) (Transformation|GetActorLocation))) 0.0) 1.0 -1.0) -8e+02) 0.0 1.5e+02) true true)
      (Class|PaperZDAnimInstance|JumptoNode (Variables|/Script/PaperZD.PaperZDAnimationComponent|GetAnimInstance (Variables|Default|GetAnimationComponent)) "damaged" "None")
      (Utilities|FlowControl|RetriggerableDelay 1.0)
      (Variables|Default|SetenemyDamaged false))))

(fn ConstructionScript)