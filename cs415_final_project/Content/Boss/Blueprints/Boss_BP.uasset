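; Boss character for a side-on game that follows the player along X to within a set range, flips to face them, and shows a health bar widget.
; A looping timer with a randomized interval triggers the attack animation, while a separate Attack event fires a projectile aimed at the player.
; Damage updates the bar, knocks the boss back, briefly blocks attacks and restores Flying movement after a delay.
; At zero health it plays death and destroys itself.
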(event Custom|HandleRotation
  ;[1 1 1] HandleRotation
  (if (not (Variables|Default|GetisDead))
    (if (< (.x (Math|Vector|GetUnitDirection(Vector) (Transformation|GetActorLocation (Game|GetPlayerCharacter 0)) (Transformation|GetActorLocation))) 0.0)
      (Transformation|SetActorRotation "0, 0, 0")
      (else
        (Transformation|SetActorRotation "0.000000,180.000000,0.000000")))))

(event Custom|playBossAttackAnimation
  (if (not (or (Variables|Default|GetenemyDamaged) (Variables|Default|GetIsDead)))
    (Class|PaperZDAnimInstance|JumptoNode (Variables|/Script/PaperZD.PaperZDAnimationComponent|GetAnimInstance (Variables|Default|GetAnimationComponent)) "attack" "None")))

(event Custom|Attack
  (Development|PrintString "Hello")
  (Transformation|SetWorldRotation (Variables|Default|GetProjectileSpawnLocation) (Math|Rotator|FindLookatRotation (Transformation|GetActorLocation) (Transformation|GetActorLocation (Game|GetPlayerCharacter 0))) false false)
  (Game|SpawnActorfromClass "/Game/Boss/Blueprints/BossProjectile_BP.BossProjectile_BP_C" (Transformation|GetWorldTransform (Variables|Default|GetProjectileSpawnLocation)) "Undefined" 0 0))

(event Collision|EventActorBeginOverlap
  (params (OtherActor :type Actor%20Object%20Reference)))

(event EventTick
  (params (DeltaSeconds :type Float%20%28single-precision%29))
  (bind _returnvalue (Transformation|GetActorLocation))
  (bind _returnvalue_2 (Game|GetPlayerCharacter 0))
  (bind _returnvalue_3 (Transformation|GetActorLocation _returnvalue_2))
  (bind _returnvalue_4 (- _returnvalue_3 _returnvalue))
  (if (not (Variables|Default|GetIsDead))
    (CallFunction|HandleRotation)
    (if (not (< (Math|Float|Absolute(Float) (.x _returnvalue_4)) 4.5e+02))
      (Pawn|Input|AddMovementInput "1.000000,0.000000,0.000000" (.x (Math|Vector|Normalize (Math|Vector|MakeVector (.x _returnvalue_4) (.y _returnvalue_4) (.z _returnvalue_4)))) false))))

(event EventBeginPlay
  (Variables|Default|SetMaxHealth (Variables|Default|GetHealth))
  (bind _returnvalue (UserInterface|CreateWidget "/Game/WidgeBlueprints/BossHealthBarWdiget.BossHealthBarWdiget_C" 0 self))
  (bind _output_get (Variables|Default|SetBossHealthRef _returnvalue))
  (UserInterface|Viewport|AddtoViewport _output_get 0)
  (bind _returnvalue_2 (Utilities|Time|SetTimerbyEvent (delegate Custom|playBossAttackAnimation) (Math|Random|RandomFloatinRange 2.0 4.0) true))
  (Variables|Default|SetbossAttackEvent _returnvalue_2))

(event Game|Damage|EventAnyDamage
  (params (Damage :type Float%20%28single-precision%29) (DamageType :type Damage%20Type%20Object%20Reference) (InstigatedBy :type Controller%20Object%20Reference) (DamageCauser :type Actor%20Object%20Reference))
  (Variables|Default|SetHealth (- (Variables|Default|GetHealth) Damage))
  (Variables|Default|SetenemyDamaged true)
  (Default|UpdateHealthBar (Variables|Default|GetBossHealthRef))
  (Character|LaunchCharacter (Math|Vector|MakeVector (* (select (< (.x (Math|Vector|GetUnitDirection(Vector) (Transformation|GetActorLocation DamageCauser) (Transformation|GetActorLocation))) 0.0) 1.0 -1.0) -8e+02) 0.0 3e+02) true true)
  (Utilities|FlowControl|Sequence
    (:then_0
      (if (<= (Variables|Default|GetHealth) 0.0)
        (Variables|Default|SetIsDead true)
        (Widget|RemovefromParent (Variables|Default|GetBossHealthRef))
        (Class|PaperZDAnimInstance|JumptoNode (Variables|/Script/PaperZD.PaperZDAnimationComponent|GetAnimInstance (Variables|Default|GetAnimationComponent)) "die" "None")
        (Utilities|FlowControl|Delay 3.0)
        (Actor|DestroyActor)
        (else
          (Class|PaperZDAnimInstance|JumptoNode (Variables|/Script/PaperZD.PaperZDAnimationComponent|GetAnimInstance (Variables|Default|GetAnimationComponent)) "Damage" "None")
          (Utilities|FlowControl|RetriggerableDelay 1.0)
          (Variables|Default|SetenemyDamaged false))))
    (:then_1
      (Utilities|FlowControl|Delay 0.7)
      (Pawn|Components|CharacterMovement|SetMovementMode (Variables|Character|GetCharacterMovement) "MOVE_Flying" 0))))

(fn ConstructionScript)